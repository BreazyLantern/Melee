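; Actor component that stores a combat character's stats, such as health, stamina and armor, as base, max and current values.
; Changes clamp between zero and max, and every current-value write broadcasts an update event.
; Stamina is the only regenerating stat, refilling on a looping timer after a retriggerable delay.
; TakeDamage reduces damage through an armor formula and sets the owner's state manager to Dead when health runs out.
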(event Custom|StartRegen
  (params (Stat%20Type :type E_Stats%20Enum :default "NewEnumerator0"))
  (switch Utilities|FlowControl|Switch|SwitchonE_Stats Stat%20Type
    (:NewEnumerator2
      (Utilities|Time|ClearTimerbyFunctionName 0 "RegenStamina")
      (Utilities|FlowControl|RetriggerableDelay 1.5)
      (Utilities|Time|SetTimerbyFunctionName 0 "RegenStamina" 0.1 true))))

(event EventBeginPlay)

(event EventTick
  (params (DeltaSeconds :type Float%20%28single-precision%29)))

(fn GetCurrentStats
  (params (Stat :type E_Stats%20Enum :default "NewEnumerator0"))
  (return (.Value (Utilities|Map|Find (Variables|Default|GetCurrentStats) Stat))))

(fn SetCurrentStats
  (params (Stat :type E_Stats%20Enum :default "NewEnumerator0") (Value :type Float%20%28double-precision%29))
  (Utilities|Map|Add (Variables|Default|GetCurrentStats) Stat Value)
  (Default|CallOnCurrentStatValueUpdated Stat Value))

(fn InitializeStats
  (bind _keys (Utilities|Map|Keys (Variables|BaseStats|GetBaseStats)))
  (for _array_element _keys
    (CallFunction|SetCurrentStats _array_element (.basevalue (.Value (Utilities|Map|Find (Variables|BaseStats|GetBaseStats) _array_element))))))

(fn ModifyCurrentStatValue
  (params (Stat :type E_Stats%20Enum :default "NewEnumerator0") (Value :type Float%20%28double-precision%29) (bShouldRegenerate :type Boolean))
  (if (!= Value 0.0)
    (bind _output_get (LocalVariables|SetL_Value (+ (CallFunction|GetCurrentStats Stat) Value)))
    (CallFunction|SetCurrentStats Stat (Math|Float|Clamp(Float) _output_get 0.0 (BaseStat|GetMaxStatValue Stat)))
    (if bShouldRegenerate
      (CallFunction|StartRegen Stat))))

(fn GetBasedStatValue
  (params (Stat :type E_Stats%20Enum :default "NewEnumerator0"))
  (return (.basevalue (.Value (Utilities|Map|Find (Variables|BaseStats|GetBaseStats) Stat)))))

(fn GetMaxStatValue
  (params (Stat :type E_Stats%20Enum :default "NewEnumerator0"))
  (return (.maxvalue (.Value (Utilities|Map|Find (Variables|BaseStats|GetBaseStats) Stat)))))

(fn SetBaseStats
  (params (Stat :type E_Stats%20Enum :default "NewEnumerator0") (Value :type Float%20%28double-precision%29))
  (bind _structout (Utilities|Struct|SetmembersinF_BaseStat (.Value (Utilities|Map|Find (Variables|BaseStats|GetBaseStats) Stat)) Value))
  (Utilities|Map|Add (Variables|BaseStats|GetBaseStats) Stat _structout))

(fn SetMaxStats
  (params (Stat :type E_Stats%20Enum :default "NewEnumerator0") (Value :type Float%20%28double-precision%29))
  (bind _structout (Utilities|Struct|SetmembersinF_BaseStat (.Value (Utilities|Map|Find (Variables|BaseStats|GetBaseStats) Stat)) Value))
  (Utilities|Map|Add (Variables|BaseStats|GetBaseStats) Stat _structout))

(fn TakeDamage
  (params (InDamage :type Float%20%28double-precision%29))
  (bind _returnvalue (Components|GetOwner))
  (bind _value (CallFunction|GetCurrentStats "NewEnumerator3"))
  (bind _returnvalue_2 (Actor|GetComponentbyClass _returnvalue "/Game/CombatSystem/Blueprints/Component/BPC_StateManagerComponent.BPC_StateManagerComponent_C"))
  (bind _returnvalue_3 (|(InDamage*(InDamage/(InDamage+Armor))) InDamage _value))
  (LocalVariables|SetL_Damage (Math|Float|Clamp(Float) _returnvalue_3 0.0 _returnvalue_3))
  (CallFunction|ModifyCurrentStatValue "NewEnumerator1" (* (LocalVariables|GetL_Damage) -1.0) true)
  (if (<= (CallFunction|GetCurrentStats "NewEnumerator1") 0.0)
    (Utilities|IsValid _returnvalue_2
      (:Is%20Valid
        (Default|SetState _returnvalue_2 "(TagName=\"Character.State.Dead\")")))))

(fn RegenStamina
  (CallFunction|SetCurrentStats "NewEnumerator2" (Math|Float|Clamp(Float) (+ (CallFunction|GetCurrentStats "NewEnumerator2") (Variables|StatRegen|GetStaminaRegenRate)) 0.0 (BaseStat|GetMaxStatValue "NewEnumerator2")))
  (if (>= (CallFunction|GetCurrentStats "NewEnumerator2") (BaseStat|GetMaxStatValue "NewEnumerator2"))
    (Utilities|Time|ClearTimerbyFunctionName 0 "RegenStamina")))