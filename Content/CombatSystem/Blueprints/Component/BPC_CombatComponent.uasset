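; Combat component that holds an actor's main weapon, combat-enabled state and attack tracking.
; Setting a new weapon unequips and destroys any valid previous one, then stores the new reference without equipping it.
; Toggling combat broadcasts the OnCombatToggled dispatcher, and ResetAttack clears the attack count and saved-attack flag.
; All logic runs through these functions, with no active BeginPlay or Tick.
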(event EventBeginPlay)

(event EventTick
  (params (DeltaSeconds :type Float%20%28single-precision%29)))

(fn SetMainWeapon
  (params (NewWeapon :type BP%20Base%20Weapon%20Object%20Reference))
  (Utilities|FlowControl|Sequence
    (:then_0
      (Utilities|IsValid (Variables|Combat|GetMainWeapon)
        (:Is%20Valid
          (Default|OnUnequipped (Variables|Combat|GetMainWeapon))
          (Actor|DestroyActor (Variables|Combat|GetMainWeapon)))))
    (:then_1
      (Variables|Combat|SetMainWeapon NewWeapon))))

(fn GetMainWeapon
  (return (Variables|Combat|GetMainWeapon)))

(fn SetCombatEnabled
  (params (EnableCombat :type Boolean))
  (Variables|Combat|SetbCombatEnabled? EnableCombat)
  (Default|CallOnCombatToggled (Variables|Combat|GetbCombatEnabled?)))

(fn IsCombatEnabled?
  (return (Variables|Combat|GetbCombatEnabled?)))

(fn ResetAttack
  (Variables|Combat|SetAttackCount 0)
  (Variables|Combat|SetbIsAttackSaved? false))