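; Actor component that gives the owning Character toggleable combat lock-on to a target.
; It sphere-traces along the follow camera for an actor implementing BPI_Targeting and notifies it when targeted or released.
; Each tick it interpolates control rotation toward the target, disabling lock-on when targeting checks fail.
; Toggling lock-on also switches movement between camera-oriented and default rotation, based on BPC_CombatComponent's combat state and speed mode.
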(event Custom|EnableLockon
  (bind (_returnvalue _targetlockto) (CallFunction|FindTarget))
  (if (and _returnvalue (CallFunction|CanTargetActor _targetlockto))
    (CallFunction|SetTargetActor _targetlockto)
    (CallFunction|SetIsTargeting true)
    (CallFunction|UpdateRotationMode)))

(event Custom|DisableLockon
  (CallFunction|SetIsTargeting false)
  (CallFunction|SetTargetActor)
  (CallFunction|UpdateRotationMode))

(event Custom|ToggleLockon
  (if (not (CallFunction|IsTargeting?))
    (CallFunction|EnableLockon)
    (else
      (CallFunction|DisableLockon))))

(event EventBeginPlay
  (Variables|Initialization|SetOwner%20Character (.AsCharacter (Utilities|Casting|CastToCharacter (Components|GetOwner))))
  (Variables|Initialization|SetOwner%20Controller (Pawn|GetController (Variables|Initialization|GetOwner%20Character)))
  (Variables|Default|SetFollow%20Cam (Actor|GetComponentbyClass (Variables|Initialization|GetOwner%20Character) "/Script/Engine.CameraComponent")))

(event EventTick
  (params (DeltaSeconds :type Float%20%28single-precision%29))
  (if (Variables|Initialization|GetbIsTargeting)
    (CallFunction|UpdateTargetingControlRotation)))

(fn SetIsTargeting
  (params (bEnableTargeting :type Boolean))
  (Variables|Initialization|SetbIsTargeting bEnableTargeting)
  (bind _followtarget (Variables|Default|GetFollowTarget)
    (:then
      (Class|BPITargeting|OnTargeted(Message) _followtarget bEnableTargeting))
    (:else)))

(fn IsTargeting?
  (return (Variables|Initialization|GetbIsTargeting)))

(fn FindTarget
  (bind _owner_character (Variables|Initialization|GetOwner%20Character))
  (bind _returnvalue (Transformation|GetActorLocation _owner_character))
  (bind (_outhit _returnvalue_2) (Collision|SphereTraceForObjects _returnvalue (+ _returnvalue (* (Math|Vector|GetForwardVector (Variables|Default|GetFollow%20Cam)) (Variables|Initialization|GetTargetingDistance))) (Variables|Initialization|GetTargetingRadius) (Variables|Initialization|GetTargetingObjectTypes) false (Utilities|Array|MakeArray (Variables|Initialization|GetOwner%20Character)) "None"))
  (if (and _returnvalue_2 (Utilities|IsValid (.HitActor (Collision|BreakHitResult _outhit))))
    (if (Utilities|DoesObjectImplementInterface (.HitActor (Collision|BreakHitResult _outhit)) "/Game/CombatSystem/Blueprints/Interfaces/BPI_Targeting.BPI_Targeting_C")
      (return true (.HitActor (Collision|BreakHitResult _outhit)))
      (else
        (return false 0)))
    (else
      (return false 0))))

(fn SetTargetActor
  (params (NewTargetActor :type Actor%20Object%20Reference))
  (Variables|Default|SetFollowTarget NewTargetActor))

(fn GetTargetActor
  (return (Variables|Default|GetFollowTarget)))

(fn UpdateTargetingControlRotation
  (bind _returnvalue (Utilities|Time|GetWorldDeltaSeconds))
  (bind _targetrotationinterpspeed (Variables|Initialization|GetTargetRotationInterpSpeed))
  (bind _owner_controller (Variables|Initialization|GetOwner%20Controller))
  (bind _owner_character (Variables|Initialization|GetOwner%20Character))
  (bind _followtarget (Variables|Default|GetFollowTarget))
  (bind _returnvalue_2 (Transformation|GetActorRotation _owner_controller))
  (bind _returnvalue_3 (Transformation|GetActorLocation _owner_character))
  (bind _returnvalue_4 (Transformation|GetActorLocation _followtarget))
  (bind _returnvalue_5 (- _returnvalue_4 "0.000000,0.000000,100.000000"))
  (bind _returnvalue_6 (Math|Rotator|FindLookatRotation _returnvalue_3 _returnvalue_5))
  (bind _returnvalue_7 (Math|Interpolation|RInterpTo _returnvalue_2 _returnvalue_6 _returnvalue _targetrotationinterpspeed))
  (bind (_roll _pitch _yaw) (Math|Rotator|BreakRotator _returnvalue_7))
  (if (and (Utilities|IsValid (Variables|Initialization|GetOwner%20Character)) (Utilities|IsValid (Variables|Initialization|GetOwner%20Controller)))
    (if (CallFunction|CanTargetActor (Variables|Default|GetFollowTarget))
      (Pawn|SetControlRotation (Variables|Initialization|GetOwner%20Controller) (Math|Rotator|MakeRotator (.Roll (Math|Rotator|BreakRotator _returnvalue_2)) _pitch _yaw))
      (else
        (CallFunction|DisableLockon)))))

(fn SetRotationMode
  (params (NewRotationMode :type E_RotationMode%20Enum :default "NewEnumerator0"))
  (bind _owner_character (Variables|Initialization|GetOwner%20Character))
  (bind _owner_character_2 (Variables|Initialization|GetOwner%20Character))
  (bind _charactermovement (Variables|/Script/Engine.Character|GetCharacterMovement _owner_character))
  (bind _charactermovement_2 (Variables|/Script/Engine.Character|GetCharacterMovement _owner_character_2))
  (bind _output_get (Variables|Default|SetCurrentRotationMode NewRotationMode))
  (switch Utilities|FlowControl|Switch|SwitchonE_RotationMode _output_get
    (:NewEnumerator0
      (Variables|/Script/Engine.CharacterMovementComponent|SetbUseControllerDesiredRotation _charactermovement_2 true)
      (Variables|/Script/Engine.CharacterMovementComponent|SetbOrientRotationToMovement _charactermovement_2 false))
    (:NewEnumerator1
      (Variables|/Script/Engine.CharacterMovementComponent|SetbUseControllerDesiredRotation _charactermovement false)
      (Variables|/Script/Engine.CharacterMovementComponent|SetbOrientRotationToMovement _charactermovement true))))

(fn GetRotationMode
  (return (Variables|Default|GetCurrentRotationMode)))

(fn CanTargetActor
  (params (Actor :type Actor%20Object%20Reference))
  (Utilities|IsValid Actor
    (:Is%20Valid
      (bind _bistargetable (Class|BPITargeting|CanbeTargeted(Message) Actor))
      (return (and _bistargetable (< (Transformation|GetDistanceTo (Components|GetOwner) (Variables|Default|GetFollowTarget)) (Variables|Initialization|GetTargetingDistance)))))
    (:Is%20Not%20Valid
      (return false))))

(fn UpdateRotationMode
  (Utilities|IsValid (Variables|Default|GetOwnerCombatCom)
    (:Is%20Valid
      _)
    (:Is%20Not%20Valid
      (Variables|Default|SetOwnerCombatCom (Actor|GetComponentbyClass (Variables|Initialization|GetOwner%20Character) "/Game/CombatSystem/Blueprints/Component/BPC_CombatComponent.BPC_CombatComponent_C"))))
  (bind _returnvalue (Class|BPICombat|GetMovementSpeedMode(Message) (Variables|Default|GetOwnerCombatCom)))
  (CallFunction|SetRotationMode (select (Math|Boolean|ANDBoolean (Default|IsCombatEnabled? (Variables|Default|GetOwnerCombatCom)) (Utilities|Enum|Equal(Enum) _returnvalue "NewEnumerator2") (CallFunction|IsTargeting?)) "NewEnumerator0" (Variables|Initialization|GetDefaultRotationMode))))