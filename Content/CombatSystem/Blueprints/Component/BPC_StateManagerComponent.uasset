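; BPC_StateManagerComponent is an actor component in the combat system that tracks the owner's current state and current character action as gameplay tags.
; Each setter ignores unchanged values, otherwise firing an end dispatcher for the old tag and a begin dispatcher for the new one.
; Getters and exact-match container checks let other code query both tags, and ResetState sets the state back to the empty default.
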(event EventBeginPlay)

(event EventTick
  (params (DeltaSeconds :type Float%20%28single-precision%29)))

(fn SetState
  (params (New%20State :type Gameplay%20Tag%20Structure))
  (if (!= New%20State (Variables|Default|GetCurrentState))
    (Default|CallOnStateEnd (Variables|Default|GetCurrentState))
    (bind _output_get (Variables|Default|SetCurrentState New%20State))
    (Default|CallOnStateBegin _output_get)))

(fn GetCurrentState
  (return (Variables|Default|GetCurrentState)))

(fn ResetState
  (State|SetState))

(fn IsCurrentStateEqualtoAny?
  (params (StateToCheck :type Gameplay%20Tag%20Container%20Structure))
  (return (GameplayTags|HasTag StateToCheck (Variables|Default|GetCurrentState) true)))

(fn SetCurrentAction
  (params (New%20Character%20Action :type Gameplay%20Tag%20Structure))
  (if (!= New%20Character%20Action (Variables|Default|GetCurrentCharacterAction))
    (Default|CallOnCharacterActionEnd (Variables|Default|GetCurrentCharacterAction))
    (bind _output_get (Variables|Default|SetCurrentCharacterAction New%20Character%20Action))
    (Default|CallOnCharacterActionBegin _output_get)))

(fn GetCurrentAction
  (return (Variables|Default|GetCurrentCharacterAction)))

(fn IsCurrentActionEqualtoAny?
  (params (ActionsToCheck :type Gameplay%20Tag%20Container%20Structure))
  (return (GameplayTags|HasTag ActionsToCheck (Variables|Default|GetCurrentCharacterAction) true)))