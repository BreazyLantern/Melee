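; Boss enemy Blueprint that extends a parent enemy class with a melee weapon and a health bar widget shown only while targeted.
; The weapon collision component traces the weapon mesh and applies directional point damage to hit actors that can receive it.
; Toggling combat snaps the weapon between hand and holster sockets.
; On death, parent logic runs and the weapon switches to simulated physics.
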(event OnHit(BPC_WeaponCollisionComponent)
  (params (Hit%20Result :type Hit%20Result%20Structure))
  (bind _hitactor (Collision|BreakHitResult Hit%20Result))
  (bind _returnvalue (Class|BPICombat|CanRecieveDamage(Message) _hitactor))
  (if _returnvalue
    (Game|Damage|ApplyPointDamage _hitactor (Variables|Initialize|GetBase%20Damage) (Transformation|GetActorForwardVector) Hit%20Result (Pawn|GetController) self (Variables|Default|GetDamagetTypeClass))
    (else
      (Development|PrintString "Is Dead"))))

(event OnCombatToggled(BPC_CombatComponent)
  (params (bIsCombatEnabled? :type Boolean))
  (Transformation|AttachComponentToComponent (Variables|Default|GetWeaponMesh) (Variables|Character|GetMesh) (select bIsCombatEnabled? (Variables|Initialize|GetWeaponHand) (Variables|Initialize|GetSocket%20Name)) "SnapToTarget" "SnapToTarget" "SnapToTarget" true))

(event Custom|SimulateWeaponPhysics
  (bind _weaponmesh (Variables|Default|GetWeaponMesh))
  (Collision|SetCollisionProfileName _weaponmesh "PhysicsActor" true :!class /Script/Engine.PrimitiveComponent)
  (Physics|SetSimulatePhysics _weaponmesh true))

(event EventBeginPlay
  (|CallParentFunction)
  (Default|SetCollisionMesh (Variables|Default|GetBPC_WeaponCollisionComponent) (Variables|Default|GetWeaponMesh))
  (bind _returnvalue (UserInterface|CreateWidget "/Game/CombatSystem/UI/WB_HealthBar.WB_HealthBar_C" (Game|GetPlayerController 0) (Variables|Default|GetBPC_StatsComponent) false))
  (UserInterface|SetWidget (Variables|Default|GetHealthBar) _returnvalue))

(event Collision|EventActorBeginOverlap
  (params (OtherActor :type Actor%20Object%20Reference)))

(event EventTick
  (params (DeltaSeconds :type Float%20%28single-precision%29)))

(event EventOnTargeted
  (params (IsTargeted? :type Boolean))
  (|CallParentFunction IsTargeted?)
  (Rendering|SetVisibility (Variables|Default|GetHealthBar) IsTargeted? false))

(event EventPerformDeath
  (|CallParentFunction)
  (CallFunction|SimulateWeaponPhysics))

(fn ConstructionScript
  (|CallParentFunction))