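; BP_MasterAI is a combat AI character, apparently the base for enemies, that attacks, reacts to hits, can be targeted and dies.
; State manager, combat, stats and weapon collision components gate and track its actions.
; Attacks and actions pick montages by gameplay tag, with attacks advancing a combo counter.
; Point damage updates stats and triggers directional stun or knockdown with impact effects, while depleted health sets Dead, ragdolling then destroying it.
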(event OnStateBegin(BPC_StateManagerComponent)
  (params (CharacterStates :type Gameplay%20Tag%20Structure))
  ;[0.4678 0 0.03245] Character States
  (|SwitchGameplayTag CharacterStates
    (:Character.State.Dead
      (CallFunction|PerformDeath))))

(event OnStateEnd(BPC_StateManagerComponent)
  (params (CharacterState :type Gameplay%20Tag%20Structure))
  ;[0.4678 0 0.03245] Character States
  (|SwitchGameplayTag CharacterState))

(event OnCurrentStatValueUpdated(BPC_StatsComponent)
  (params (StatType :type E_Stats%20Enum :default "NewEnumerator0") (Value :type Float%20%28double-precision%29))
  ;[0.4678 0 0.03245] Stats
  (if (and (Utilities|Enum|Equal(Enum) StatType "NewEnumerator1") (<= Value 0.0))
    (Default|SetState (Variables|Default|GetBPC_StateManagerComponent) "(TagName=\"Character.State.Dead\")")))

(event Custom|Attack%20Event
  ;[0.4678 0 0.03245] Attacking
  (if (Attack|CanPerformAttack?)
    (CallFunction|PerformCombatAttack (CallFunction|GetDesiredAttackType) (Variables|/Game/CombatSystem/Blueprints/Component/BPC_CombatComponent.BPC_CombatComponent_C|GetAttackCount (Variables|Default|GetBPC_CombatComponent)) false)))

(event Custom|ApplyHitReaction
  (params (InDamageType :type E_DamageType%20Enum :default "NewEnumerator0"))
  ;[0.4678 0 0.03245] HitEffects
  (switch Utilities|FlowControl|Switch|SwitchonE_DamageType InDamageType
    (:NewEnumerator0
      (CallFunction|PerformHitStun :!label _label))
    (:NewEnumerator1
      (goto _label))
    (:NewEnumerator2
      (CallFunction|PerformKnockDown))))

(event Custom|PerformDeath
  ;[0.4678 0 0.03245] Character States
  (TakeDamage|EnableRagdoll)
  (TakeDamage|ApplyHitReactionPhysicsVelocity 2e+03)
  (Utilities|FlowControl|Delay 4.0)
  (Actor|DestroyActor))

(event Custom|ApplyImpactEffect
  (params (InDamageType :type E_DamageType%20Enum :default "NewEnumerator0"))
  (bind _last_hit_info (Variables|Default|GetLast%20Hit%20Info))
  (bind _location (Collision|BreakHitResult _last_hit_info))
  ;[0.4678 0 0.03245] HitEffects
  (switch Utilities|FlowControl|Switch|SwitchonE_DamageType InDamageType
    (:NewEnumerator0
      _)
    (:NewEnumerator1
      _)
    (:NewEnumerator2
      _))
  (Audio|PlaySoundatLocation "/Game/CombatSystem/CourseFiles/SoundFX/Gruntling/Impact/A_Guardian_Impact_Cue.A_Guardian_Impact_Cue" _location "0, 0, 0" 1.0 1.0 0.0 0 0 0 0)
  (Effects|SpawnEmitteratLocation "/Game/Realistic_Starter_VFX_Pack_Vol2/Particles/Blood/P_Blood_Splat_Cone.P_Blood_Splat_Cone" _location))

(event EventContinueAttack
  ;[0.4678 0 0.03245] Attacking
  (if (Variables|/Game/CombatSystem/Blueprints/Component/BPC_CombatComponent.BPC_CombatComponent_C|GetbIsAttackSaved? (Variables|Default|GetBPC_CombatComponent))
    (Variables|/Game/CombatSystem/Blueprints/Component/BPC_CombatComponent.BPC_CombatComponent_C|SetbIsAttackSaved? (Variables|Default|GetBPC_CombatComponent) false)
    (if (== (Default|GetCurrentState (Variables|Default|GetBPC_StateManagerComponent)) "(TagName=\"Character.State.Attacking\")")
      (Default|ResetState (Variables|Default|GetBPC_StateManagerComponent)))
    (CallFunction|AttackEvent)))

(event EventBeginPlay
  ;[0.4678 0 0.03245] Being Play
  (Default|InitializeStats (Variables|Default|GetBPC_StatsComponent)))

(event EventResetAttack
  ;[0.4678 0 0.03245] Attacking
  (Default|ResetAttack (Variables|Default|GetBPC_CombatComponent)))

(event EventResetCombat
  ;[0.4678 0 0.03245] Combat Reset
  (Default|ResetAttack (Variables|Default|GetBPC_CombatComponent))
  (Default|ResetState (Variables|Default|GetBPC_StateManagerComponent))
  (Default|SetCurrentAction (Variables|Default|GetBPC_StateManagerComponent)))

(event EventOnTargeted
  (params (IsTargeted? :type Boolean))
  (Rendering|SetVisibility (Variables|Default|GetTargetingWidget) IsTargeted? false))

(event Game|Damage|EventPointDamage
  (params (Damage :type Float%20%28single-precision%29) (DamageType :type Damage%20Type%20Object%20Reference) (HitLocation :type Vector :default "0, 0, 0") (HitNormal :type Vector :default "0, 0, 0") (HitComponent :type Primitive%20Component%20Object%20Reference) (BoneName :type Name :default "None") (ShotFromDirection :type Vector :default "0, 0, 0") (InstigatedBy :type Controller%20Object%20Reference) (DamageCauser :type Actor%20Object%20Reference) (HitInfo :type Hit%20Result%20Structure%20%28by%20ref%29))
  (bind _returnvalue (Pawn|GetControlledPawn InstigatedBy))
  ;[0.4678 0 0.03245] Damage
  (bind _asbp_attack_damage_type (Utilities|Casting|CastToBP_AttackDamageType DamageType))
  (Variables|Default|SetbHitFront (Math|Float|InRange(Float) (Class|Actor|GetDotProductto _returnvalue self) -0.1 1.0))
  (Variables|Default|SetLast%20Hit%20Info HitInfo)
  (Default|TakeDamage (Variables|Default|GetBPC_StatsComponent) Damage)
  (Class|AISenseDamage|ReportDamageEvent self _returnvalue Damage HitLocation HitLocation "None")
  (if (TakeDamage|CanRecieveHitReaction?)
    (CallFunction|ApplyHitReaction (Variables|/Game/CombatSystem/Blueprints/DamageTypes/BP_AttackDamageType.BP_AttackDamageType_C|GetDamageType _asbp_attack_damage_type))
    (CallFunction|ApplyImpactEffect (Variables|/Game/CombatSystem/Blueprints/DamageTypes/BP_AttackDamageType.BP_AttackDamageType_C|GetDamageType _asbp_attack_damage_type))))

(event EventActivateCollision
  (params (CPart :type E_CollisionPart%20Enum :default "NewEnumerator0"))
  (Default|EnableCollision (Variables|Default|GetBPC_WeaponCollisionComponent)))

(event EventDeactivateCollision
  (params (CPart :type E_CollisionPart%20Enum :default "NewEnumerator0"))
  (Default|DisableCollision (Variables|Default|GetBPC_WeaponCollisionComponent)))

(event EventToggleCombat
  (bind _bpc_combatcomponent (Variables|Default|GetBPC_CombatComponent))
  (Default|SetCombatEnabled _bpc_combatcomponent (not (Default|IsCombatEnabled? _bpc_combatcomponent))))

(event Input|KeyboardEvents|Tab
  (params (Key :type Key%20Structure :default "None"))
  (:Pressed
    (Default|ModifyCurrentStatValue (Variables|Default|GetBPC_StatsComponent) "NewEnumerator1" -5e+01 true)))

(fn ConstructionScript
  (bind _capsulecomponent (Variables|Collision|GetCapsuleComponent))
  (bind _relativelocation (Variables|/Script/Engine.SceneComponent|GetRelativeLocation _capsulecomponent))
  (bind (_x _y _z) (Math|Vector|BreakVector _relativelocation))
  ;[0 0.2131 1] Exact heigt placement of mesh to capsule. Is a preference
  (Transformation|SetWorldLocation (Variables|Character|GetMesh) (Math|Vector|MakeVector _x _y (- _z (Variables|/Script/Engine.CapsuleComponent|GetCapsuleHalfHeight _capsulecomponent))) false false)
  (Default|InitializeStats (Variables|Default|GetBPC_StatsComponent)))

(fn CanPerformToggleCombat?
  (return (and (not (Default|IsCurrentStateEqualtoAny? (Variables|Default|GetBPC_StateManagerComponent) "(GameplayTags=((TagName=\"Character.State.Attacking\"),(TagName=\"Character.State.Dead\"),(TagName=\"Character.State.Disabled\"),(TagName=\"Character.State.Dodging\"),(TagName=\"Character.State.GeneralAction\")))")) (not (AI|Components|NavMovement|IsFalling (Variables|Character|GetCharacterMovement))))))

(fn CanPerformAttack?
  (return (and (not (Default|IsCurrentStateEqualtoAny? (Variables|Default|GetBPC_StateManagerComponent) "(GameplayTags=((TagName=\"Character.State.Attacking\"),(TagName=\"Character.State.Dead\"),(TagName=\"Character.State.Disabled\"),(TagName=\"Character.State.Dodging\"),(TagName=\"Character.State.GeneralAction\")))")) (>= (Default|GetCurrentStats (Variables|Default|GetBPC_StatsComponent) "NewEnumerator2") 1e+01))))

(fn CanPerformDodge?
  (return (Math|Boolean|ANDBoolean (not (Default|IsCurrentStateEqualtoAny? (Variables|Default|GetBPC_StateManagerComponent) "(GameplayTags=((TagName=\"Character.State.Dead\"),(TagName=\"Character.State.Disabled\"),(TagName=\"Character.State.Dodging\"),(TagName=\"Character.State.GeneralAction\")))")) (not (AI|Components|NavMovement|IsFalling (Variables|Character|GetCharacterMovement))) (>= (Default|GetCurrentStats (Variables|Default|GetBPC_StatsComponent) "NewEnumerator2") 1e+01))))

(fn EnableRagdoll
  (bind _returnvalue (Utilities|Name|MakeLiteralName "pelvis"))
  (Pawn|Components|CharacterMovement|SetMovementMode (Variables|Character|GetCharacterMovement) "MOVE_None" 0)
  (Collision|SetCollisionResponsetoChannel (Variables|Collision|GetCapsuleComponent) "ECC_Pawn" "ECR_Ignore")
  (Collision|SetCollisionResponsetoChannel (Variables|Collision|GetCapsuleComponent) "ECC_Camera" "ECR_Ignore")
  (Collision|SetCollisionProfileName (Variables|Character|GetMesh) "ragdoll" true :!class /Script/Engine.PrimitiveComponent)
  (Class|SkeletalMeshComponent|SetAllBodiesBelowSimulatePhysics (Variables|Character|GetMesh) _returnvalue true true)
  (Class|SkeletalMeshComponent|SetAllBodiesBelowPhysicsBlendWeight (Variables|Character|GetMesh) _returnvalue 1.0 false true))

(fn ApplyHitReactionPhysicsVelocity
  (params (InitialSpeed :type Float%20%28double-precision%29))
  (Physics|SetPhysicsLinearVelocity (Variables|Character|GetMesh) (* (Transformation|GetActorForwardVector) (* InitialSpeed -1.0)) false "pelvis"))

(fn CanJump?
  (return (and (not (Default|IsCurrentStateEqualtoAny? (Variables|Default|GetBPC_StateManagerComponent) "(GameplayTags=((TagName=\"Character.State.Dead\"),(TagName=\"Character.State.Disabled\"),(TagName=\"Character.State.Dodging\"),(TagName=\"Character.State.GeneralAction\")))")) (not (AI|Components|NavMovement|IsFalling (Variables|Character|GetCharacterMovement))))))

(fn CanRecieveHitReaction?
  (return (not (Default|IsCurrentStateEqualtoAny? (Variables|Default|GetBPC_StateManagerComponent) "(GameplayTags=((TagName=\"Character.State.Dead\")))"))))

(fn SetMovementSpeedMode
  (params (NewSpeedMode :type E_MovementSpeed%20Enum :default "NewEnumerator0"))
  (if (Utilities|Enum|NotEqual(Enum) NewSpeedMode (Variables|MovementSpeeds|GetMovementSpeedMode))
    (bind _output_get (Variables|MovementSpeeds|SetMovementSpeedMode NewSpeedMode))
    (switch Utilities|FlowControl|Switch|SwitchonE_MovementSpeed _output_get
      (:NewEnumerator0
        (Variables|/Script/Engine.CharacterMovementComponent|SetMaxWalkSpeed (Variables|Character|GetCharacterMovement) (Variables|MovementSpeeds|GetMax%20Walk%20Speed)))
      (:NewEnumerator1
        (Variables|/Script/Engine.CharacterMovementComponent|SetMaxWalkSpeed (Variables|Character|GetCharacterMovement) (Variables|MovementSpeeds|GetMax%20Jog%20Speed)))
      (:NewEnumerator2
        (Variables|/Script/Engine.CharacterMovementComponent|SetMaxWalkSpeed (Variables|Character|GetCharacterMovement) (Variables|MovementSpeeds|GetMax%20Sprint%20Speed))))))

(fn GetCurrentSpeedMode
  (return (Variables|MovementSpeeds|GetMovementSpeedMode)))

(fn GetDesiredAttackType
  (if (AI|Components|NavMovement|IsFalling (Variables|Character|GetCharacterMovement))
    (return "(TagName=\"Character.Action.Attack.FallingAttack\")")
    (elif (Utilities|Enum|Equal(Enum) (MovementSpeeds|GetCurrentSpeedMode) "NewEnumerator2")
      (return "(TagName=\"Character.Action.Attack.SprintAttack\")")
      (else
        (return "(TagName=\"Character.Action.Attack.LightAttack\")")))))

(fn CanPerformSprint
  (return (!= (Math|Vector|VectorLength (Transformation|GetVelocity)) 0.0)))

(fn PerformHitStun
  (bind _output_get (LocalVariables|SetL_HitMontage (select (Variables|Default|GetbHitFront) (Variables|Montages|GetHitReactionFrontMontage) (Variables|Montages|GetHitReacttionBack))))
  (Utilities|IsValid _output_get
    (:Is%20Valid
      (Animation|PlayAnimMontage (LocalVariables|GetL_HitMontage) 1.0 "None")
      (Default|SetState (Variables|Default|GetBPC_StateManagerComponent) "(TagName=\"Character.State.Disabled\")"))
    (:Is%20Not%20Valid
      (return))))

(fn PerformKnockDown
  (Animation|PlayAnimMontage (Variables|Montages|GetKnockDownFrontMontage) 1.0 "None")
  (Default|SetState (Variables|Default|GetBPC_StateManagerComponent) "(TagName=\"Character.State.Disabled\")"))

(fn GetActionMontage
  (params (ActionTag :type Gameplay%20Tag%20Structure))
  (|SwitchGameplayTag ActionTag
    (:Character.Action.Attack.CloseRange
      (return (Variables|Montages|GetCloseRangeAttack)))
    (:Character.Action.Dodge
      (return (Variables|Montages|GetDodgeMontages)))
    (:Character.Action.EnterCombat
      (return (Utilities|Array|MakeArray (Variables|Montages|GetEnterCombat))))
    (:Character.Action.ExitCombat
      (return (Utilities|Array|MakeArray (Variables|Montages|GetExitCombat))))
    (:Character.Action.Attack.MidRange
      (return (Variables|Montages|GetMidRangeMontage)))))

(fn CanbeTargeted
  (return (!= (Default|GetCurrentState (Variables|Default|GetBPC_StateManagerComponent)) "(TagName=\"Character.State.Dead\")")))

(fn CanRecieveDamage
  (return (not (Default|IsCurrentStateEqualtoAny? (Variables|Default|GetBPC_StateManagerComponent) "(GameplayTags=((TagName=\"Character.State.Dead\")))"))))

(fn GetDesiredRotation
  (if (Utilities|Operators|NotEqual(!=) :A (Pawn|Components|PawnMovement|GetLastInputVector (Variables|Character|GetCharacterMovement)) :ErrorTolerance 0.0001)
    (return (Math|Conversions|RotationFromXVector (Class|Pawn|GetLastMovementInputVector)))
    (else
      (return (Transformation|GetActorRotation)))))

(fn GetMovementSpeedMode
  (return (MovementSpeeds|GetCurrentSpeedMode)))

(fn PerformCombatAction
  (params (ActionTag :type Gameplay%20Tag%20Structure) (StateTag :type Gameplay%20Tag%20Structure) (MontageIndex :type Integer) (bRandomIndex :type Boolean))
  (LocalVariables|SetL_ActionMontages (CallFunction|GetActionMontage ActionTag))
  (bind _output_get (LocalVariables|SetL_ActionMontage (select bRandomIndex (.OutItem (Utilities|Array|Random (LocalVariables|GetL_ActionMontages))) (Utilities|Array|Get(acopy) (LocalVariables|GetL_ActionMontages) (select (> MontageIndex (Utilities|Array|LastIndex (LocalVariables|GetL_ActionMontages))) 0 MontageIndex)))))
  (Utilities|IsValid _output_get
    (:Is%20Valid
      (Default|SetState (Variables|Default|GetBPC_StateManagerComponent) StateTag)
      (Default|SetCurrentAction (Variables|Default|GetBPC_StateManagerComponent) ActionTag)
      (bind _returnvalue (Animation|PlayAnimMontage (LocalVariables|GetL_ActionMontage) 1.0 "None"))
      (return _returnvalue))
    (:Is%20Not%20Valid
      (return 0.0))))

(fn PerformCombatAttack
  (params (AttackType :type Gameplay%20Tag%20Structure) (Index :type Integer) (bRandomIndex :type Boolean))
  (LocalVariables|SetL_AttackMontages (CallFunction|GetActionMontage AttackType))
  (bind _output_get (LocalVariables|SetL_AttackMontage (select bRandomIndex (.OutItem (Utilities|Array|Random (LocalVariables|GetL_AttackMontages))) (Utilities|Array|Get(acopy) (LocalVariables|GetL_AttackMontages) (select (> Index (Utilities|Array|LastIndex (LocalVariables|GetL_AttackMontages))) 0 Index)))))
  (Utilities|IsValid _output_get
    (:Is%20Valid
      (Default|SetState (Variables|Default|GetBPC_StateManagerComponent) "(TagName=\"Character.State.Attacking\")")
      (Default|SetCurrentAction (Variables|Default|GetBPC_StateManagerComponent) AttackType)
      (bind _returnvalue (Animation|PlayAnimMontage (LocalVariables|GetL_AttackMontage) 1.0 "None"))
      (LocalVariables|SetAttackDuration _returnvalue)
      (bind _result (Math|Integer|IncrementInt (Variables|/Game/CombatSystem/Blueprints/Component/BPC_CombatComponent.BPC_CombatComponent_C|GetAttackCount (Variables|Default|GetBPC_CombatComponent)))
        (:%20%20
          (if (> _result (Utilities|Array|LastIndex (LocalVariables|GetL_AttackMontages)))
            (Variables|/Game/CombatSystem/Blueprints/Component/BPC_CombatComponent.BPC_CombatComponent_C|SetAttackCount (Variables|Default|GetBPC_CombatComponent) 0))
          (return (LocalVariables|GetAttackDuration)))))
    (:Is%20Not%20Valid
      (Development|PrintString "Montage Not Valid" true true "(R=0.467784,G=0.000000,B=0.032447,A=1.000000)")
      (return 0.0))))