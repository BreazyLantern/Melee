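; BP_BaseWeapon is an equippable weapon base that supplies combat montages, stat costs and damage to its owner.
; On equip it attaches to a hand or stowed socket, registers with the combat component, updates the anim instance's combat type and configures its collision component.
; Collision hits apply point damage, scaled by the state manager's current action, to targets that can receive it.
; Montages are selected by gameplay tag, though Falling Attack returns none.
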(event OnHit(BPC_CollisionComponent)
  (params (Hit%20Result :type Hit%20Result%20Structure))
  (bind _hitactor (Collision|BreakHitResult Hit%20Result))
  (bind _returnvalue (Class|BPICombat|CanRecieveDamage(Message) _hitactor))
  (if _returnvalue
    (Game|Damage|ApplyPointDamage _hitactor (Stat|GetDamage) (Transformation|GetActorForwardVector (Components|GetOwner)) Hit%20Result (Game|GetInstigatorController) self)
    (else
      (Development|PrintString "Is Dead"))))

(event Custom|SimulateWeaponPhysics
  (bind _mesh (CallFunction|GetItemMesh))
  (Collision|SetCollisionProfileName _mesh "PhysicsActor" true :!class /Script/Engine.PrimitiveComponent)
  (Physics|SetSimulatePhysics _mesh true))

(event EventBeginPlay
  (|CallParentFunction) ; This node is disabled and will not be called.\nDrag off pins to build functionality.
)

(event Collision|EventActorBeginOverlap
  (params (OtherActor :type Actor%20Object%20Reference))
  (|CallParentFunction OtherActor) ; This node is disabled and will not be called.\nDrag off pins to build functionality.
)

(event EventTick
  (params (DeltaSeconds :type Float%20%28single-precision%29))
  (|CallParentFunction DeltaSeconds) ; This node is disabled and will not be called.\nDrag off pins to build functionality.
)

(fn ConstructionScript
  (|CallParentFunction))

(fn OnEquipped
  (|CallParentFunction)
  (Variables|Default|SetCombatComponent (Actor|GetComponentbyClass (Components|GetOwner) "/Game/CombatSystem/Blueprints/Component/BPC_CombatComponent.BPC_CombatComponent_C"))
  (Variables|Default|SetOwnerStateManager (Actor|GetComponentbyClass (Components|GetOwner) "/Game/CombatSystem/Blueprints/Component/BPC_StateManagerComponent.BPC_StateManagerComponent_C"))
  (CallFunction|AttachActor (select (Default|IsCombatEnabled? (Variables|Default|GetCombatComponent)) (Variables|Initialization|GetHandSocketName) (Variables|Default|GetAttachedSocketName)))
  (Default|SetMainWeapon (Variables|Default|GetCombatComponent) self)
  (Class|BPIAnimInstance|UpdateCombatType(Message) (Components|SkeletalMesh|GetAnimInstance (Variables|/Script/Engine.Character|GetMesh (.AsCharacter (Utilities|Casting|CastToCharacter (Components|GetOwner))))) (Variables|Initialization|GetCombatType))
  (Default|SetCollisionMesh (Variables|Default|GetBPC_CollisionComponent) (CallFunction|GetItemMesh))
  (Default|AddActortoIgnore (Variables|Default|GetBPC_CollisionComponent) (Components|GetOwner)))

(fn GetActionMontages
  (params (Index :type Gameplay%20Tag%20Structure))
  (|SwitchGameplayTag Index
    (:Character.Action.Attack.LightAttack
      (return (Variables|Montages|GetLightAttackMontages)))
    (:Character.Action.Attack.StrongAttack
      (return (Variables|Montages|GetHeavyAttackMontages)))
    (:Character.Action.Attack.ChargedAttack
      (return (Variables|Montages|GetCharged%20Attack%20Montages)))
    (:Character.Action.Attack.SprintAttack
      (return (Variables|Montages|GetSprint%20Attack%20Montages)))
    (:Character.Action.Attack.FallingAttack
      (return 0))
    (:Character.Action.Dodge
      (return (Variables|Montages|GetDodgeMontages)))
    (:Character.Action.EnterCombat
      (return (Utilities|Array|MakeArray (Variables|Montages|GetEnterCombat))))
    (:Character.Action.ExitCombat
      (return (Utilities|Array|MakeArray (Variables|Montages|GetExitCombat))))))

(fn GetStatCostforAction
  (bind _ownerstatemanager (Variables|Default|GetOwnerStateManager)
    (:then
      (return (.Value (Utilities|Map|Find (Variables|Stat|GetActionStatCost) (Default|GetCurrentAction _ownerstatemanager)))))
    (:else
      (return 0.0))))

(fn GetDamage
  (bind _ownerstatemanager (Variables|Default|GetOwnerStateManager)
    (:then
      (return (* (Variables|Stat|GetDamage) (Math|Float|Clamp(Float) (.Value (Utilities|Map|Find (Variables|Stat|GetActionDamageMult) (Default|GetCurrentAction _ownerstatemanager))) 1.0 (.Value (Utilities|Map|Find (Variables|Stat|GetActionDamageMult) (Default|GetCurrentAction _ownerstatemanager)))))))
    (:else
      (return (Variables|Stat|GetDamage)))))